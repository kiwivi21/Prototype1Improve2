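; BP_Gun is the player's hitscan gun, which fires a line trace from the first-person camera to hit targets.
; It caches the first-person character on BeginPlay, and FireBullet fetches it again if that reference is invalid.
; CheckForCollision traces forward from the camera on the Visibility channel, and FireBullet calls BecomeHit on any hit actor derived from BP_ParentTarget.
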(event `self.ReceiveBeginPlay`
  (bind _asbp_first_person_character (cast `/Game/FirstPerson/Blueprints/BP_FirstPersonCharacter` (`GameplayStatics.GetPlayerCharacter` 0)))
  (set `self.PlayerRef` _asbp_first_person_character))

(event `FireBullet`
  (`/Engine/EditorBlueprintResources/StandardMacros.IsValid` (`self.PlayerRef`)
    (:`Is Valid`
      _)
    (:`Is Not Valid`
      (bind _asbp_first_person_character (cast `/Game/FirstPerson/Blueprints/BP_FirstPersonCharacter` (`GameplayStatics.GetPlayerCharacter` 0)))
      (set `self.PlayerRef` _asbp_first_person_character)))
  (bind (_returnvalue _hitresult) (`self.CheckForCollision`))
  (if _returnvalue
    (bind _asbp_parent_target (cast `/Game/Blueprints/TargetsOREnemies/BP_ParentTarget` (`.HitActor` (`GameplayStatics.BreakHitResult` _hitresult))))
    (`/Game/Blueprints/TargetsOREnemies/BP_ParentTarget.BecomeHit` _asbp_parent_target)))

(fn `CheckForCollision`
  (returns (ReturnValue :type Boolean) (HitResult :type "HitResult Structure"))
  (bind _firstpersoncamera (`/Game/FirstPerson/Blueprints/BP_FirstPersonCharacter.FirstPersonCamera` (`self.PlayerRef`)))
  (bind _returnvalue (`SceneComponent.K2_GetComponentLocation` _firstpersoncamera))
  (bind _returnvalue_2 (`SceneComponent.GetForwardVector` _firstpersoncamera))
  (bind (_outhit _returnvalue_3) (`KismetSystemLibrary.LineTraceSingle` (+ _returnvalue (* _returnvalue_2 1.0)) (+ _returnvalue (* _returnvalue_2 5000.0)) "TraceTypeQuery1"))
  (return _returnvalue_3 _outhit))

(fn `UserConstructionScript`)