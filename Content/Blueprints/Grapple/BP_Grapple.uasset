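; Grappling hook gun actor that pulls the first-person player toward whatever surface the hook hits.
; Firing line-traces from the player camera, attaches the Hook to the hit actor and shows the Cable; releasing snaps it back to the gun.
; While attached, Tick adds pull velocity toward the hook onto the clamped player velocity in Falling mode and aims the gun at the hit point.
; The same trace runs every Tick to drive the crosshair's in-range state.
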(event `self.ReceiveBeginPlay`
  ;[0 0 1] Set player ref
  (bind _asbp_first_person_character (cast `/Game/FirstPerson/Blueprints/BP_FirstPersonCharacter` (`GameplayStatics.GetPlayerCharacter` 0)))
  (set `self.PlayerRef` _asbp_first_person_character)
  (set `self.DefaultGunRotation` (`SceneComponent.K2_GetComponentRotation` (`self.Gun`))))

(event `FireGrapple`
  ;[0 0 1] Fire grapple
  (`self.PlayerRef`
    (:`then`
      _)
    (:`else`
      (bind _asbp_first_person_character (cast `/Game/FirstPerson/Blueprints/BP_FirstPersonCharacter` (`GameplayStatics.GetPlayerCharacter` 0)))
      (bind _output_get (set `self.PlayerRef` _asbp_first_person_character))))
  (bind (_returnvalue _hitresult) (`self.CheckForCollision`))
  (if _returnvalue
    (bind (_bblockinghit _binitialoverlap _time _distance _location _impactpoint _normal _impactnormal _physmat _hitactor) (`GameplayStatics.BreakHitResult` _hitresult))
    (set `self.HitLocation` _location)
    (set `self.HitActor` _hitactor)
    (`SceneComponent.K2_SetWorldLocationAndRotation` (`self.Hook`) (`self.HitLocation`) (`KismetMathLibrary.Conv_VectorToRotator` (`KismetMathLibrary.GreaterGreater_VectorRotator` (0.0 90.0 0.0) (`SceneComponent.K2_GetComponentRotation` (`/Game/FirstPerson/Blueprints/BP_FirstPersonCharacter.FirstPersonCamera` (`self.PlayerRef`))))) false false)
    (`SceneComponent.K2_AttachToComponent` (`self.Hook`) (`Actor.RootComponent` (`self.HitActor`)) "None" "KeepWorld" "KeepWorld" "KeepWorld" true)
    (`SceneComponent.SetVisibility` (`self.Cable`) true false)
    (set `self.GrappleAttached` true)
    (`GameplayStatics.PlaySound2D` "/Game/Assets/SFX/Grapple/StartGrapple2.StartGrapple2" 1.0 1.0 0.0 null null)))

(event `ReleaseGrapple`
  ;[0 0 1] Release the grapple
  (set `self.GrappleAttached` false)
  (`SceneComponent.SetVisibility` (`self.Cable`) false false)
  (`CharacterMovementComponent.SetMovementMode` (`Character.CharacterMovement` (`self.PlayerRef`)) "MOVE_Falling" 0)
  (`SceneComponent.K2_SetRelativeRotation` :`self` (`self.Gun`))
  (`SceneComponent.K2_AttachToComponent` (`self.Hook`) (`self.HookScene`) "None" "SnapToTarget" "SnapToTarget" "SnapToTarget" true)
  (`GameplayStatics.PlaySound2D` "/Game/Assets/SFX/Grapple/EndGrapple.EndGrapple" 1.0 0.0 0.0 null null))

(event `self.ReceiveTick`
  (params (DeltaSeconds :type "Float (single-precision)"))
  (bind _gun (`self.Gun`))
  (bind _currentwidget (`/Game/FirstPerson/Blueprints/BP_FirstPersonCharacter.CurrentWidget` (`self.PlayerRef`)))
  ;[1 0 0.01384] Control for dynamic crosshair
  (bind _returnvalue (`self.CheckForCollision`))
  (if _returnvalue
    (set `/Game/Blueprints/UI/BP_Crosshair.In_Range` true _currentwidget)
    (else
      (set `/Game/Blueprints/UI/BP_Crosshair.In_Range` false _currentwidget)))
  ;[0 0 1] Pull player
  (if (`self.GrappleAttached`)
    (set `MovementComponent.Velocity` (+ (* (`KismetMathLibrary.GetDirectionUnitVector` (`SceneComponent.K2_GetComponentLocation` (`self.Gun`)) (`SceneComponent.K2_GetComponentLocation` (`self.Hook`))) (`self.PullStrength`)) (`KismetMathLibrary.ClampVectorSize` (`self.GetVelocity` (`self.PlayerRef`)) 0.0 6000.0)) (`Character.CharacterMovement` (`self.PlayerRef`)))
    (`CharacterMovementComponent.SetMovementMode` (`Character.CharacterMovement` (`self.PlayerRef`)) "MOVE_Falling" 0)
    (`SceneComponent.K2_SetWorldRotation` _gun (`KismetMathLibrary.FindLookAtRotation` (`SceneComponent.K2_GetComponentLocation` _gun) (`self.HitLocation`)) false false)))

(fn `CheckForCollision`
  (returns (ReturnValue :type Boolean) (HitResult :type "HitResult Structure"))
  (bind _firstpersoncamera (`/Game/FirstPerson/Blueprints/BP_FirstPersonCharacter.FirstPersonCamera` (`self.PlayerRef`)))
  (bind _returnvalue (`SceneComponent.K2_GetComponentLocation` _firstpersoncamera))
  (bind _returnvalue_2 (`SceneComponent.GetForwardVector` _firstpersoncamera))
  (bind (_outhit _returnvalue_3) (`KismetSystemLibrary.LineTraceSingle` (+ _returnvalue (* _returnvalue_2 1.0)) (+ _returnvalue (* _returnvalue_2 10000.0)) "TraceTypeQuery1"))
  (return _returnvalue_3 _outhit))

(fn `UserConstructionScript`)