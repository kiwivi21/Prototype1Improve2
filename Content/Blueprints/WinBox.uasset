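; WinBox is a level-completion trigger actor that ends play with a win screen when any actor overlaps it, with no check on which actor.
; On overlap it pauses the game, switches to UI-only input with a visible cursor, and creates a focused WBP_WinScreen, calling its GetMedal with itself.
; It then removes the first-person character's current widget and plays the YouWin sound.
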(event `self.ReceiveActorBeginOverlap`
  (params (OtherActor :type "Actor Object Reference"))
  (bind _returnvalue (`GameplayStatics.GetPlayerController` 0))
  (`GameplayStatics.SetGamePaused` true)
  (`WidgetBlueprintLibrary.SetInputMode_UIOnlyEx` _returnvalue null "DoNotLock" true)
  (set `PlayerController.bShowMouseCursor` true _returnvalue)
  (bind _returnvalue_2 (`|CreateWidget` "/Game/Blueprints/UI/WBP_WinScreen.WBP_WinScreen_C" _returnvalue))
  (`UserWidget.AddToViewport` _returnvalue_2 0)
  (`Widget.SetKeyboardFocus` _returnvalue_2)
  (`/Game/Blueprints/UI/WBP_WinScreen.GetMedal` _returnvalue_2 self)
  (bind _asbp_first_person_character (cast `/Game/FirstPerson/Blueprints/BP_FirstPersonCharacter` (`GameplayStatics.GetPlayerCharacter` 0)))
  (`Widget.RemoveFromParent` (`/Game/FirstPerson/Blueprints/BP_FirstPersonCharacter.CurrentWidget` _asbp_first_person_character))
  (`GameplayStatics.PlaySound2D` "/Game/Assets/SFX/Music/YouWin.YouWin" 1.0 1.0 0.0 null null)
  (`GameplayStatics.SetGamePaused` true))

(fn `UserConstructionScript`)